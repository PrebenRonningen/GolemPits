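; BP_Projectile is a test bullet actor that turns homing shortly after spawning.
; On BeginPlay it sets movement velocity from its Velocity vector times initial speed and sweeps a short step forward along that direction.
; Tick accumulates lifetime, then once past a brief delay enables homing toward HomingTargetComponent on its ProjectileMovement.
; The actor destroys itself when its Bullet component hits anything.
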(event OnComponentHit(Bullet)
  (params (HitComponent :type Primitive%20Component%20Object%20Reference) (OtherActor :type Actor%20Object%20Reference) (OtherComp :type Primitive%20Component%20Object%20Reference) (NormalImpulse :type Vector :default "0, 0, 0") (Hit :type Hit%20Result%20Structure%20%28by%20ref%29))
  (Actor|DestroyActor))

(event EventBeginPlay
  (bind _projectilemovement (Variables|Default|GetProjectileMovement))
  (Variables|/Script/Engine.MovementComponent|SetVelocity _projectilemovement (* (Variables|Default|GetVelocity) (Variables|/Script/Engine.ProjectileMovementComponent|GetInitialSpeed _projectilemovement)))
  (Transformation|SetActorLocation (+ (Transformation|GetActorLocation) (* (Variables|Default|GetVelocity) 2e+01)) true false))

(event EventTick
  (params (DeltaSeconds :type Float%20%28single-precision%29))
  (if (< 0.3 (Variables|Default|GetLifetime))
    (Utilities|FlowControl|DoOnce false
      (:Completed
        (Variables|/Script/Engine.ProjectileMovementComponent|SetbIsHomingProjectile (Variables|Default|GetProjectileMovement) true)
        (Variables|/Script/Engine.ProjectileMovementComponent|SetHomingTargetComponent (Variables|Default|GetProjectileMovement) (Variables|Default|GetHoming%20Target%20Component))))
    (else
      (Variables|Default|SetLifetime (+ DeltaSeconds (Variables|Default|GetLifetime))))))

(fn ConstructionScript)