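; BP_Projectile_Nature is a thorn projectile that flies along a given direction and expires on impact or timeout.
; On BeginPlay it scales its Velocity variable by the ProjectileMovement component's initial speed to set the launch velocity.
; Tick counts down Lifetime and destroys the actor once it drops below zero, while a hit on the Thorn component destroys it immediately, with no damage logic in this graph.
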(event OnComponentHit(Thorn)
  (params (HitComponent :type Primitive%20Component%20Object%20Reference) (OtherActor :type Actor%20Object%20Reference) (OtherComp :type Primitive%20Component%20Object%20Reference) (NormalImpulse :type Vector :default "0, 0, 0") (Hit :type Hit%20Result%20Structure%20%28by%20ref%29))
  (Actor|DestroyActor))

(event EventTick
  (params (DeltaSeconds :type Float%20%28single-precision%29))
  (bind _output_get (Variables|Default|SetLifetime (- (Variables|Default|GetLifetime) DeltaSeconds)))
  (if (< _output_get 0.0)
    (Actor|DestroyActor)))

(event EventBeginPlay
  (bind _projectilemovement (Variables|Default|GetProjectileMovement))
  (Variables|/Script/Engine.MovementComponent|SetVelocity _projectilemovement (* (Variables|Default|GetVelocity) (Variables|/Script/Engine.ProjectileMovementComponent|GetInitialSpeed _projectilemovement))))

(fn ConstructionScript)