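; BP_IceCone is a placed ice cone actor that links to another cone in range with an ice wall.
; On BeginPlay it searches other cones in reverse array order and stops at the first within MinRange in 2D.
; It spawns a BP_IceWall at their midpoint, rotated and X-scaled to span the gap, cross-references all three and flags both cones connected.
; Tick counts down LifeTime on unconnected cones and destroys them at zero.
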(event EventBeginPlay
  (bind _cone (Variables|Default|GetCone))
  (bind _returnvalue (Transformation|GetWorldLocation _cone))
  (bind _outactors (Actor|GetAllActorsOfClass "BP_IceCone_C"))
  (bind _array_index (Utilities|Array|ForEachLoopwithBreak _outactors :!label _label)
    (:LoopBody
      (if (!= (Utilities|Array|Get(acopy) _outactors (- (- (Utilities|Array|Length _outactors) 1) _array_index)) self)
        (if (< (Math|Vector2D|Vector2DLength (- (Math|Vector2D|MakeVector2D (.x (Transformation|GetActorLocation (Utilities|Array|Get(acopy) _outactors (- (- (Utilities|Array|Length _outactors) 1) _array_index)))) (.y (Transformation|GetActorLocation (Utilities|Array|Get(acopy) _outactors (- (- (Utilities|Array|Length _outactors) 1) _array_index))))) (Math|Conversions|ToVector2D(Vector) (Transformation|GetWorldLocation (Variables|Default|GetCone))))) (Variables|Default|GetMinRange))
          (bind _returnvalue_2 (Game|SpawnActorfromClass "/Game/Test/TestingGround/BP_IceWall.BP_IceWall_C" (Math|Transform|MakeTransform (Math|Vector|Lerp(Vector) (Math|Vector|MakeVector (.x (Transformation|GetActorLocation (Utilities|Array|Get(acopy) _outactors (- (- (Utilities|Array|Length _outactors) 1) _array_index)))) (.y (Transformation|GetActorLocation (Utilities|Array|Get(acopy) _outactors (- (- (Utilities|Array|Length _outactors) 1) _array_index)))) (.z (Transformation|GetActorLocation (Utilities|Array|Get(acopy) _outactors (- (- (Utilities|Array|Length _outactors) 1) _array_index))))) _returnvalue 0.5) (Math|Rotator|MakeRotfromX (Math|Vector|Normalize (- (Math|Vector|MakeVector (.x (Transformation|GetActorLocation (Utilities|Array|Get(acopy) _outactors (- (- (Utilities|Array|Length _outactors) 1) _array_index)))) (.y (Transformation|GetActorLocation (Utilities|Array|Get(acopy) _outactors (- (- (Utilities|Array|Length _outactors) 1) _array_index)))) (.z (Transformation|GetActorLocation (Utilities|Array|Get(acopy) _outactors (- (- (Utilities|Array|Length _outactors) 1) _array_index))))) _returnvalue))) (Math|Vector|MakeVector (/ (Math|Vector2D|Vector2DLength (- (Math|Vector2D|MakeVector2D (.x (Transformation|GetActorLocation (Utilities|Array|Get(acopy) _outactors (- (- (Utilities|Array|Length _outactors) 1) _array_index)))) (.y (Transformation|GetActorLocation (Utilities|Array|Get(acopy) _outactors (- (- (Utilities|Array|Length _outactors) 1) _array_index))))) (Math|Conversions|ToVector2D(Vector) (Transformation|GetWorldLocation (Variables|Default|GetCone))))) 1e+02) 1.0 1.0)) "Undefined" self 0))
          (Variables|/Game/Test/TestingGround/BP_IceWall.BP_IceWall_C|SetCones _returnvalue_2 (Utilities|Array|MakeArray (Utilities|Array|Get(acopy) _outactors (- (- (Utilities|Array|Length _outactors) 1) _array_index)) self))
          (Utilities|Array|Add (Variables|BP_IceCone_C|GetIceWalls (Utilities|Array|Get(acopy) _outactors (- (- (Utilities|Array|Length _outactors) 1) _array_index))) _returnvalue_2)
          (Utilities|Array|Add (Variables|Default|GetIceWalls) _returnvalue_2)
          (bind _output_get (Variables|BP_IceCone_C|SetIsConnected (Utilities|Array|Get(acopy) _outactors (- (- (Utilities|Array|Length _outactors) 1) _array_index)) true))
          (Variables|Default|SetIsConnected _output_get)
          (goto _label Break))))))

(event Collision|EventActorBeginOverlap
  (params (OtherActor :type Actor%20Object%20Reference)))

(event EventTick
  (params (DeltaSeconds :type Float%20%28single-precision%29))
  (if (not (Variables|Default|GetIsConnected))
    (bind _output_get (Variables|Default|SetLifeTime (- (Variables|Default|GetLifeTime) DeltaSeconds)))
    (if (<= _output_get 0.0)
      (Actor|DestroyActor))))

(fn ConstructionScript)