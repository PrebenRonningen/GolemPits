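; BP_TargetMarker is a target marker actor with a TargetWidget that tracks and exposes a locked-on state.
; On BeginPlay it binds to the widget's LockedOn event, which sets the IsLockedOn flag returned by GetIsLockedOn.
; Each Tick it rotates to face its owner and scales uniformly with distance to that owner within a clamped range, so the marker grows as the owner moves away.
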(event Custom|LockedOn
  (Variables|Private|SetIsLockedOn true))

(event EventTick
  (params (DeltaSeconds :type Float%20%28single-precision%29))
  (bind _returnvalue (Components|GetOwner))
  (bind _self self)
  (bind _returnvalue_2 (Transformation|GetDistanceTo _returnvalue))
  (bind _returnvalue_3 (+ _returnvalue_2 1e+03))
  (bind _returnvalue_4 (/ _returnvalue_3 1.5e+03))
  (bind _returnvalue_5 (Math|Float|Clamp(Float) _returnvalue_4 1.0 3.0))
  (Transformation|SetActorRotation _self (Math|Conversions|RotationFromXVector (Math|Vector|GetUnitDirection(Vector) (Transformation|GetActorLocation _self) (Transformation|GetActorLocation _returnvalue))))
  (Transformation|SetActorScale3D (Math|Vector|MakeVector _returnvalue_5 _returnvalue_5 _returnvalue_5)))

(event EventBeginPlay
  (bind _astarget_widget (Utilities|Casting|CastToTargetWidget (UserInterface|GetUserWidgetObject (Variables|Default|GetTargetMarkerWidget))))
  (EventDispatchers|BindEventtoLockedon _astarget_widget (delegate Custom|LockedOn)))

(fn ConstructionScript)

(fn GetIsLockedon
  (return (Variables|Private|GetIsLockedOn)))