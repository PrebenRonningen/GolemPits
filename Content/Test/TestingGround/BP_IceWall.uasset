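; BP_IceWall is a temporary ice wall actor that grows upward and removes itself when its lifetime ends.
; Tick increases the static mesh's Z scale at GrowSpeed until it reaches MaxReach, while counting down LifeTime.
; On expiry, it destroys linked Cones that no other wall shares, removes itself from the surviving cones' IceWalls lists, then destroys itself.
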(event EventBeginPlay)

(event Collision|EventActorBeginOverlap
  (params (OtherActor :type Actor%20Object%20Reference)))

(event EventTick
  (params (DeltaSeconds :type Float%20%28single-precision%29))
  (bind _staticmesh (Variables|Default|GetStaticMesh))
  (bind _cones (Variables|Default|GetCones))
  (bind _returnvalue (Transformation|GetWorldScale _staticmesh))
  (Utilities|FlowControl|Sequence
    (:then_0
      (if (< (.z _returnvalue) (Variables|Default|GetMaxReach))
        (Transformation|SetWorldScale3D _staticmesh (Math|Vector|MakeVector (.x _returnvalue) (.y _returnvalue) (+ (.z _returnvalue) (* (Variables|Default|GetGrowSpeed) DeltaSeconds))))))
    (:then_1
      (bind _output_get (Variables|Default|SetLifeTime (- (Variables|Default|GetLifeTime) DeltaSeconds)))
      (if (<= _output_get 0.0)
        (for _array_element _cones
          (if (not (> (Utilities|Array|Length (Variables|/Game/Test/TestingGround/BP_IceCone.BP_IceCone_C|GetIceWalls _array_element)) 1))
            (Actor|DestroyActor _array_element)))
        (for _array_element_2 _cones
          (Utilities|IsValid _array_element_2
            (:Is%20Valid
              (Utilities|Array|RemoveItem (Variables|/Game/Test/TestingGround/BP_IceCone.BP_IceCone_C|GetIceWalls _array_element_2) self))))
        (Actor|DestroyActor)))))

(fn ConstructionScript)